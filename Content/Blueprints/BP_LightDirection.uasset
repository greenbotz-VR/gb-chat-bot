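; BP_LightDirection is an actor that publishes a light direction vector as the LightVector parameter, apparently in a Material Parameter Collection.
; SetupMPC converts the forward vector of its Arrow component's world rotation to a linear color and writes it to that parameter.
; It runs from the construction script, BeginPlay, every Tick and a custom event, so the value follows the actor's rotation.
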(event `self.ReceiveBeginPlay`
  (`self.SetupMPC` :!label _label))

(event `bp_Event`
  (goto _label))

(event `self.ReceiveTick`
  (params (DeltaSeconds :type "Float (single-precision)"))
  (goto _label))

(fn `SetupMPC`
  (`KismetMaterialLibrary.SetVectorParameterValue` null "LightVector" (`KismetMathLibrary.Conv_VectorToLinearColor` (`KismetMathLibrary.Conv_RotatorToVector` (`SceneComponent.K2_GetComponentRotation` (`self.Arrow`))))))

(fn `UserConstructionScript`
  (`self.SetupMPC`))