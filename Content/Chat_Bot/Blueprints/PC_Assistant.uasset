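; PC_Assistant is the player controller Blueprint in the Chat_Bot folder, setting up the on-screen interface at startup.
; On BeginPlay it creates the UI_main widget, keeps a reference to it, adds it to the viewport and shows the mouse cursor.
; A disconnected graph compares the mouse position with stored values to flag movement, but it never runs and Tick is empty.
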(event `self.ReceiveBeginPlay`
  (bind _returnvalue (`|CreateWidget` "/Game/Chat_Bot/Blueprints/Widgets/UI_main.UI_main_C" (`GameplayStatics.GetPlayerController` 0)))
  (bind _output_get (set `self.UI` _returnvalue))
  (`UserWidget.AddToViewport` _output_get 0)
  (set `self.bShowMouseCursor` true))

(event `self.ReceiveTick`
  (params (DeltaSeconds :type "Float (single-precision)")))

(fn `UserConstructionScript`)