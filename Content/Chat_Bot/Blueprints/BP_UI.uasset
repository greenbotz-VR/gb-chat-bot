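; BP_UI is an actor that owns the main UI widget for the chatbot project and toggles it on a key press.
; On BeginPlay it creates UI_main, adds it to the viewport hidden, and enables input for the first player controller.
; Pressing S flips between showing the widget with the mouse cursor and hiding both, using a FlipFlop.
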(event `self.ReceiveBeginPlay`
  (bind _returnvalue (`|CreateWidget` "/Game/Chat_Bot/Blueprints/Widgets/UI_main.UI_main_C"))
  (bind _output_get (set `self.UI_main` _returnvalue))
  (`UserWidget.AddToViewport` _output_get 0)
  (`Widget.SetVisibility` _output_get "Hidden")
  (`self.EnableInput` (`GameplayStatics.GetPlayerController` 0)))

(event `Key|S`
  (params (Key :type "Key Structure"))
  (bind _returnvalue (`GameplayStatics.GetPlayerController` 0))
  (bind _ui_main (`self.UI_main`))
  (:`Pressed`
    (`/Engine/EditorBlueprintResources/StandardMacros.FlipFlop`
      (:`A`
        (set `PlayerController.bShowMouseCursor` true _returnvalue)
        (`Widget.SetVisibility` _ui_main "Visible"))
      (:`B`
        (set `PlayerController.bShowMouseCursor` false _returnvalue)
        (`Widget.SetVisibility` _ui_main "Hidden")))))

(fn `UserConstructionScript`)