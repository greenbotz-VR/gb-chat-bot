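; BP_Wall is a wall enclosure with right, left, top and back pieces that can be resized by width, height and depth.
; WallAdjustment nudges each piece outward by world-space offsets, moving the side walls in opposite directions along X.
; SetWallAdjustment places them at absolute world coordinates, mirroring the sides around world X zero rather than the actor's origin.
; The event graph and construction script are empty, so resizing relies on calls to these functions.
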(event `self.ReceiveBeginPlay`)

(event `self.ReceiveActorBeginOverlap`
  (params (OtherActor :type "Actor Object Reference")))

(event `self.ReceiveTick`
  (params (DeltaSeconds :type "Float (single-precision)")))

(fn `Set_Wall_Adjustment`
  (params (Width :type "Float (double-precision)") (Height :type "Float (double-precision)") (Depth :type "Float (double-precision)"))
  (bind _r_wall (`self.R_Wall`))
  (bind _l_wall (`self.L_Wall`))
  (bind _top_wall (`self.Top_Wall`))
  (bind _back_wall (`self.Back_Wall`))
  (`|ExecutionSequence`
    (:`then_0`
      (`SceneComponent.K2_SetWorldLocation` _r_wall (`KismetMathLibrary.MakeVector` Width (.y (`SceneComponent.K2_GetComponentLocation` _r_wall)) (.z (`SceneComponent.K2_GetComponentLocation` _r_wall))) false false)
      (`SceneComponent.K2_SetWorldLocation` _l_wall (`KismetMathLibrary.MakeVector` (- 0.0 Width) (.y (`SceneComponent.K2_GetComponentLocation` _l_wall)) (.z (`SceneComponent.K2_GetComponentLocation` _l_wall))) false false))
    (:`then_1`
      (`SceneComponent.K2_SetWorldLocation` _top_wall (`KismetMathLibrary.MakeVector` (.x (`SceneComponent.K2_GetComponentLocation` _top_wall)) (.y (`SceneComponent.K2_GetComponentLocation` _top_wall)) Height) false false))
    (:`then_2`
      (`SceneComponent.K2_SetWorldLocation` _back_wall (`KismetMathLibrary.MakeVector` (.x (`SceneComponent.K2_GetComponentLocation` _back_wall)) (- 0.0 Depth) (.z (`SceneComponent.K2_GetComponentLocation` _back_wall))) false false))))

(fn `UserConstructionScript`)

(fn `Wall_Adjustment`
  (params (Wall_Width :type "Float (double-precision)") (Wall_Height :type "Float (double-precision)") (Wall_Depth :type "Float (double-precision)"))
  (bind _returnvalue (+ Wall_Width 0.0))
  (`|ExecutionSequence`
    (:`then_0`
      (`SceneComponent.K2_AddWorldOffset` (`self.R_Wall`) (`KismetMathLibrary.MakeVector` _returnvalue) false false)
      (`SceneComponent.K2_AddWorldOffset` (`self.L_Wall`) (- (0.0 0.0 0.0) (`KismetMathLibrary.MakeVector` _returnvalue)) false false))
    (:`then_1`
      (`SceneComponent.K2_AddWorldOffset` (`self.Top_Wall`) (`KismetMathLibrary.MakeVector` 0.0 0.0 Wall_Height) false false))
    (:`then_2`
      (`SceneComponent.K2_AddWorldOffset` (`self.Back_Wall`) (`KismetMathLibrary.MakeVector` 0.0 (- 0.0 Wall_Depth)) false false))))