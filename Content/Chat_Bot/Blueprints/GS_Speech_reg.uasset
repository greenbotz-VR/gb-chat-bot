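; GS_Speech_reg is a chat bot actor Blueprint that switches on keyword-based speech recognition when play begins.
; It passes the phrase list in CusPrases to the SpeechRecognitionSubsystem, then prints the first phrase and its tolerance on screen as a debug check.
; A grammar mode call is left unconnected, and the graph has no handler for recognized phrases.
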(event `self.ReceiveBeginPlay`
  (bind (_phrase _tolerance) (break `RecognitionPhrase` (`|GetArrayItem` (`.Elements_5_9ACF689C498A7761F957A094691B0384` (break `/Game/Chat_Bot/Blueprints/Struct/STR_Phrases` (`self.Cus_Prases`))))))
  (bind _output_get (set `self.Cus_Prases` (`self.Cus_Prases`)))
  (`SpeechRecognitionSubsystem.EnableKeywordMode` (subsystem `SpeechRecognitionSubsystem`) (`.Elements_5_9ACF689C498A7761F957A094691B0384` (break `/Game/Chat_Bot/Blueprints/Struct/STR_Phrases` _output_get)))
  (`KismetSystemLibrary.PrintString` _phrase true true (struct :`R` 0.954992 :`B` 1.0 :`A` 1.0))
  (`KismetSystemLibrary.PrintString` (`|GetEnumeratorNameAsString` _tolerance) true true (struct :`R` 1.0 :`B` 0.829131 :`A` 1.0)))

(fn `UserConstructionScript`)